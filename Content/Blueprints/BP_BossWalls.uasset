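; BP_BossWalls is a toggleable rock barrier, apparently for boss encounters, that blocks passage while active.
; Activate spawns a rock particle system, plays a rumble sound, sets the box collision to block all channels, then pauses the effect after three seconds so it stays frozen in place.
; Reset sets the box to ignore all channels and destroys the particle component.
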(event `self.ReceiveBeginPlay`)

(event `Reset`
  (bind _rockfx (`self.RockFX`))
  (`PrimitiveComponent.SetCollisionResponseToAllChannels` (`self.Box`) "ECR_Ignore")
  (`/Engine/EditorBlueprintResources/StandardMacros.IsValid` _rockfx
    (:`Is Valid`
      (`ActorComponent.K2_DestroyComponent` _rockfx))))

(event `Activate`
  (bind _returnvalue (`NiagaraFunctionLibrary.SpawnSystemAtLocation` "/Game/Effects/Niagra/P_BossWalls.P_BossWalls" (`self.K2_GetActorLocation`)))
  (set `self.RockFX` _returnvalue)
  (`PrimitiveComponent.SetCollisionResponseToAllChannels` (`self.Box`) "ECR_Block")
  (`GameplayStatics.PlaySoundAtLocation` "/Game/Sounds/Monster/S_RockyRocks_Cue.S_RockyRocks_Cue" (`self.K2_GetActorLocation`) (struct) 1.0 1.0 0.0 null null null)
  (`KismetSystemLibrary.Delay` 3.0)
  (`NiagaraComponent.SetPaused` (`self.RockFX`) true))

(fn `UserConstructionScript`)