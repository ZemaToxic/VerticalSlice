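; LevelTransition is a player interactable that moves the game to another level when activated.
; Its Activate event checks the Enabled flag and casts the current game mode to BP_GM_Base.
; If that cast succeeds, it has the game mode store game data, then opens the level named by NextLevel.
; BeginPlay, overlap and Tick are unused, so the transition runs only through Activate.
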(event `self.Activate`
  (if (`self.Enabled`)
    (bind _asbp_gm_base (cast `/Game/Blueprints/BP_GM_Base` (`GameplayStatics.GetGameMode`)))
    (`/Game/Blueprints/BP_GM_Base.Store Game Data` _asbp_gm_base)
    (`GameplayStatics.OpenLevel` (`self.NextLevel`))))

(fn `UserConstructionScript`
  (`parent.UserConstructionScript`))