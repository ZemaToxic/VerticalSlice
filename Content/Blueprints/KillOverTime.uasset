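; KillOverTime is a hazard actor that kills overlapping third-person characters instantly and damages mechs over time.
; When a MechBoi2 begins overlapping, it stores that mech and starts a looping timer that applies DamageAmount each tick while health remains above zero.
; The timer is cleared when a mech leaves the overlap, the stored reference becomes invalid or its health runs out.
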(event `StartMechDamageTimer`
  (bind _returnvalue (`KismetSystemLibrary.K2_SetTimerDelegate` (delegate `DamageMech`) (`self.Time`) true))
  (set `self.Damage` _returnvalue))

(event `self.ReceiveActorBeginOverlap`
  (params (OtherActor :type "Actor Object Reference"))
  (bind _asmech_boi_2 (cast `/Game/Blueprints/Player/MechBoi2` OtherActor)
    (:`then`
      (set `self.Mech` _asmech_boi_2)
      (`self.StartMechDamageTimer`))
    (:`CastFailed`
      (bind _asthird_person_character (cast `/Game/Blueprints/Player/ThirdPersonCharacter` OtherActor))
      (`/Game/Blueprints/Player/ThirdPersonCharacter.Kill` _asthird_person_character))))

(event `DamageMech`
  (bind _mech (`self.Mech`))
  (`/Engine/EditorBlueprintResources/StandardMacros.IsValid` _mech
    (:`Is Valid`
      (if (> (`Mech.CurrentHealth` _mech) 0.0)
        (`Mech.Damage` _mech (`self.DamageAmount`) (0.0 0.0 0.0))
        (else
          (`self.StopMechDamageOverTime` :!label _label))))
    (:`Is Not Valid`
      (goto _label))))

(event `self.ReceiveActorEndOverlap`
  (params (OtherActor :type "Actor Object Reference"))
  (cast `/Game/Blueprints/Player/MechBoi2` OtherActor)
  (`self.StopMechDamageOverTime`))

(event `StopMechDamageOverTime`
  (set `self.Mech` null)
  (`KismetSystemLibrary.K2_ClearAndInvalidateTimerHandle` (`self.Damage`)))

(fn `UserConstructionScript`)