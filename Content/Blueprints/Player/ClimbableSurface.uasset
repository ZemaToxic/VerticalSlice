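; ClimbableSurface is an actor that switches climbing on and off for a ThirdPersonCharacter overlapping it.
; On overlap begin, it calls SetClimbing, enabling climbing only if the character's origin is below the top of the surface's bounds.
; The forward and up vectors it passes derive from a zero rotator, so they are world axes regardless of the actor's rotation.
; Ending overlap disables climbing with zero vectors.
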(event `self.ReceiveActorBeginOverlap`
  (params (OtherActor :type "Actor Object Reference"))
  (bind (_origin _boxextent) (`self.GetActorBounds` false))
  (bind _asthird_person_character (cast `/Game/Blueprints/Player/ThirdPersonCharacter` OtherActor))
  (bind (_returnvalue_x _returnvalue_y _returnvalue_z) (`KismetMathLibrary.BreakVector` (`self.K2_GetActorLocation` _asthird_person_character)))
  (if (> (+ (.z _origin) (.z _boxextent)) _returnvalue_z)
    (`/Game/Blueprints/Player/ThirdPersonCharacter.SetClimbing` _asthird_person_character true (`KismetMathLibrary.GetForwardVector` (struct)) (`KismetMathLibrary.GetUpVector` (struct)))
    (else
      (`/Game/Blueprints/Player/ThirdPersonCharacter.SetClimbing` _asthird_person_character false (0.0 0.0 0.0) (0.0 0.0 0.0)))))

(event `self.ReceiveActorEndOverlap`
  (params (OtherActor :type "Actor Object Reference"))
  (bind _asthird_person_character (cast `/Game/Blueprints/Player/ThirdPersonCharacter` OtherActor))
  (`/Game/Blueprints/Player/ThirdPersonCharacter.SetClimbing` _asthird_person_character false (0.0 0.0 0.0) (0.0 0.0 0.0)))

(fn `UserConstructionScript`)