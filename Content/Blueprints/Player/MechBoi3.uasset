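; Player-pilotable mech character that adds HUD, quest switching and feedback on top of its parent's aim, damage and dismount logic.
; It creates HUD and quest widgets, swaps reticles when aiming, and eases the camera via the nearer side point on mount.
; Looping timers force dismount at zero health, drive low-health warning audio and apply laser-ground damage.
; Keys 1 and 2 step the active quest, with a hardcoded QuestC1.1-to-QuestD1 handoff.
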(event `Begin Game`
  (params (Spawnpoint :type "Vector Structure") (SpawnRot :type "Rotator Structure"))
  ;[1 1 1] For level streaming
  (`self.K2_SetActorLocationAndRotation` Spawnpoint SpawnRot)
  (`ActorComponent.Activate` (`self.CharacterMovement`) false))

(event `self.ReceiveBeginPlay`
  ;[1 1 1] Add UI to the Screen
  (`AudioComponent.Stop` (`self.Audio`))
  (bind _returnvalue (`|CreateWidget` "/Game/UI/Widget_HUD.Widget_HUD_C" (`GameplayStatics.GetPlayerController` 0)))
  (bind _output_get (set `self.MainWidget` _returnvalue))
  (`UserWidget.AddToViewport` _output_get 0)
  (`self.SetMainVisability` false)
  (bind _returnvalue_2 (`|CreateWidget` "/QuestPlugin/QuestUI.QuestUI_C" (`GameplayStatics.GetPlayerController` 0)))
  (bind _output_get_2 (set `self.QuestWidget` _returnvalue_2))
  (`UserWidget.AddToViewport` _output_get_2 0)
  ;[1 1 1] Health Check
  (bind _returnvalue_3 (`KismetSystemLibrary.K2_SetTimerDelegate` (delegate `HealthChack`) 0.01 true))
  (set `self.DeathCheck` _returnvalue_3)
  (set `self.DefaultCamTrans` (`SceneComponent.GetRelativeTransform` (`self.FollowCamera`)))
  (`KismetSystemLibrary.K2_SetTimer` null "CheckLaserDamage" 0.2 true))

(event `HealthChack`
  ;[1 1 1] Health Check
  (if (and (<= (`self.CurrentHealth`) 0.0) (== (`GameplayStatics.GetPlayerPawn` 0) self))
    (`self.Dismount`)
    (`GameplayStatics.SpawnSound2D` "/Game/Sounds/Mech/S_Impact.S_Impact" 1.0 1.0 0.0 null)
    (elif (and (<= (`self.CurrentHealth`) (* (`self.MaxHealth`) (`self.HealthWarningThreshold`))) (not (`AudioComponent.IsPlaying` (`self.Audio`))))
      (`AudioComponent.Play` (`self.Audio`) 0.0)
      (elif (`AudioComponent.IsPlaying` (`self.Audio`))
        (`AudioComponent.Stop` (`self.Audio`))))))

(event `self.Aim`
  (bind _mainwidget (`self.MainWidget`))
  ;[1 1 1] Aiming UI
  (`parent.Aim`)
  (`Widget.SetVisibility` (`/Game/UI/Widget_HUD.ReticleWide` _mainwidget) "Hidden")
  (`Widget.SetVisibility` (`/Game/UI/Widget_HUD.Reticle` _mainwidget) "Visible"))

(event `Key|One`
  (params (Key :type "Key Structure"))
  ;[1 1 1] Quest Switching
  (:`Pressed`
    (bind _asbp_gm_base (cast `/Game/Blueprints/BP_GM_Base` (`GameplayStatics.GetGameMode`)))
    (bind _quest_manager (`/Game/Blueprints/BP_GM_Base.Quest Manager` _asbp_gm_base))
    (`/Engine/EditorBlueprintResources/StandardMacros.IsValid` _quest_manager
      (:`Is Valid`
        (bind _skip (`self.CheckQuest` _quest_manager))
        (if (not _skip)
          (`QuestManager.setActiveQuest` _quest_manager (- (`QuestManager.ActiveQuestId` _quest_manager) 1)))))))

(event `self.StopAim`
  (bind _mainwidget (`self.MainWidget`))
  ;[1 1 1] Aiming UI
  (`parent.StopAim`)
  (`Widget.SetVisibility` (`/Game/UI/Widget_HUD.ReticleWide` _mainwidget) "Visible")
  (`Widget.SetVisibility` (`/Game/UI/Widget_HUD.Reticle` _mainwidget) "Hidden"))

(event `Key|Two`
  (params (Key :type "Key Structure"))
  ;[1 1 1] Quest Switching
  (:`Pressed`
    (bind _asbp_gm_base (cast `/Game/Blueprints/BP_GM_Base` (`GameplayStatics.GetGameMode`)))
    (bind _quest_manager (`/Game/Blueprints/BP_GM_Base.Quest Manager` _asbp_gm_base))
    (`/Engine/EditorBlueprintResources/StandardMacros.IsValid` _quest_manager
      (:`Is Valid`
        (bind _skip (`self.CheckQuest` _quest_manager))
        (if (not _skip)
          (`QuestManager.setActiveQuest` _quest_manager (+ (`QuestManager.ActiveQuestId` _quest_manager) 1)))))))

(event `self.Damage`
  (params (dmg :type "Float (single-precision)") (Loc :type "Vector Structure"))
  ;[1 1 1] Damage Sounds
  (`GameplayStatics.SpawnEmitterAtLocation` null Loc (`KismetMathLibrary.FindLookAtRotation` (`self.K2_GetActorLocation`) Loc))
  (`parent.Damage` dmg Loc)
  (if (== (`KismetMathLibrary.RandomIntegerInRange` 0 1) 0)
    (`GameplayStatics.PlaySoundAtLocation` "/Game/Sounds/Mech/S_Hit1.S_Hit1" Loc (struct) 1.0 1.0 0.0 null null null)
    (`GameplayStatics.PlaySoundAtLocation` "/Game/Sounds/Mech/S_Impact2.S_Impact2" Loc (struct) 1.0 1.0 0.0 null null null)
    (else
      (`GameplayStatics.PlaySoundAtLocation` "/Game/Sounds/Mech/S_Hit2.S_Hit2" Loc (struct) 1.0 1.0 0.0 null null null)
      (`GameplayStatics.PlaySoundAtLocation` "/Game/Sounds/Mech/S_Impact2.S_Impact2" Loc (struct) 1.0 1.0 0.0 null null null))))

(event `self.Mount`
  (bind (_defaultcamtrans_location _defaultcamtrans_rotation) (`KismetMathLibrary.BreakTransform` (`self.DefaultCamTrans`)))
  (bind (_returnvalue_location _returnvalue_rotation) (`KismetMathLibrary.BreakTransform` (`SceneComponent.GetRelativeTransform` (`self.RightCamPos`))))
  (bind (_returnvalue_location_2 _returnvalue_rotation_2) (`KismetMathLibrary.BreakTransform` (`SceneComponent.GetRelativeTransform` (`self.LeftCamPos`))))
  (bind _relativelocation (`SceneComponent.RelativeLocation` (`self.FollowCamera`)))
  ;[1 1 1] Mount Animation Stuff
  (if (<= (`KismetMathLibrary.VSizeSquared` (- _relativelocation (`SceneComponent.RelativeLocation` (`self.RightCamPos`)))) (`KismetMathLibrary.VSizeSquared` (- _relativelocation (`SceneComponent.RelativeLocation` (`self.LeftCamPos`)))))
    (`KismetSystemLibrary.MoveComponentTo` (`self.FollowCamera`) _returnvalue_location _returnvalue_rotation true false 2.0)
    (else
      (`KismetSystemLibrary.MoveComponentTo` (`self.FollowCamera`) _returnvalue_location_2 _returnvalue_rotation_2 true false 2.0)))
  (`KismetSystemLibrary.MoveComponentTo` (`self.FollowCamera`) _defaultcamtrans_location _defaultcamtrans_rotation false true 2.0)
  (`self.SetMainVisability` true))

(event `self.Dismount`
  (`self.SetMainVisability` false)
  (`parent.Dismount`))

(event `SetMainVisability`
  (params (isVisable :type Boolean))
  (if isVisable
    (`Widget.SetVisibility` (`self.MainWidget`) "Visible")
    (else
      (`Widget.SetVisibility` (`self.MainWidget`) "Hidden"))))

(event `CheckLaserDamage`
  (if (> (`KismetArrayLibrary.Array_Length` (`PrimitiveComponent.GetOverlappingActors` (`self.CapsuleComponent`) "/Game/Blueprints/Monsters/BP_LaserGround.BP_LaserGround_C")) 0)
    (`self.Damage` 10.0 (`self.K2_GetActorLocation`))))

(event `SetQuestVisibility`
  (params (`Is Visible` :type Boolean))
  (if `Is Visible`
    (`Widget.SetVisibility` (`self.QuestWidget`) "Visible")
    (else
      (`Widget.SetVisibility` (`self.QuestWidget`) "Hidden"))))

(fn `CheckQuest`
  (params (QuestManager :type "QuestManager Object Reference"))
  (returns (Skip :type Boolean))
  (if (and (== (`QuestManager.ActiveQuestName` QuestManager) "QuestC1.1") (== (`ActiveQuest.getStage` (`QuestManager.ActiveQuest` QuestManager)) 8))
    (`ActiveQuest.addToValue` (`QuestManager.ActiveQuest` QuestManager) 0 1.0)
    (`QuestManager.setActiveQuest_Name` QuestManager "QuestD1")
    (return true)
    (else
      (return false))))

(fn `UserConstructionScript`)