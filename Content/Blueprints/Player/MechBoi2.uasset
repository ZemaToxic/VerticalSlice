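; Player mech character Blueprint that adds HUD, quest UI, camera and feedback on top of its parent class.
; BeginPlay creates both widgets and starts a fast looping timer that polls health, triggering the GameMode's end screen on death.
; Aiming swaps reticles, damage plays random hit sounds, and keys 1/2 cycle the QuestManager's active quest.
; Mounting swings the camera via the nearer side position back to default and shows the UI; dismounting hides it.
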(event `Begin Game`
  (params (Spawnpoint :type "Vector Structure") (SpawnRot :type "Rotator Structure"))
  ;[1 1 1] For level streaming
  (`self.K2_SetActorLocationAndRotation` Spawnpoint SpawnRot)
  (`ActorComponent.Activate` (`self.CharacterMovement`) false))

(event `self.ReceiveBeginPlay`
  ;[1 1 1] Add UI to the Screen
  (bind _returnvalue (`|CreateWidget` "/Game/UI/Widget_HUD.Widget_HUD_C" (`GameplayStatics.GetPlayerController` 0)))
  (bind _output_get (set `self.MainWidget` _returnvalue))
  (`UserWidget.AddToViewport` _output_get 0)
  (bind _returnvalue_2 (`|CreateWidget` "/QuestPlugin/QuestUI.QuestUI_C" (`GameplayStatics.GetPlayerController` 0)))
  (bind _output_get_2 (set `self.QuestWidget` _returnvalue_2))
  (`UserWidget.AddToViewport` _output_get_2 0)
  ;[1 1 1] Health Check
  (bind _returnvalue_3 (`KismetSystemLibrary.K2_SetTimerDelegate` (delegate `HealthChack`) 0.01 true))
  (set `self.DeathCheck` _returnvalue_3)
  (set `self.DefaultCamTrans` (`SceneComponent.GetRelativeTransform` (`self.FollowCamera`))))

(event `HealthChack`
  ;[1 1 1] Health Check
  (if (<= (`self.CurrentHealth`) 0.0)
    (bind _asbp_gm_base (cast `/Game/Blueprints/BP_GM_Base` (`GameplayStatics.GetGameMode`)))
    (`/Game/Blueprints/BP_GM_Base.EndScreen` _asbp_gm_base false)
    (`KismetSystemLibrary.K2_ClearAndInvalidateTimerHandle` (`self.DeathCheck`))))

(event `self.Aim`
  (bind _mainwidget (`self.MainWidget`))
  ;[1 1 1] Aiming UI
  (`parent.Aim`)
  (`Widget.SetVisibility` (`/Game/UI/Widget_HUD.ReticleWide` _mainwidget) "Hidden")
  (`Widget.SetVisibility` (`/Game/UI/Widget_HUD.Reticle` _mainwidget) "Visible"))

(event `Key|One`
  (params (Key :type "Key Structure"))
  ;[1 1 1] Quest Switching
  (:`Pressed`
    (bind _asbp_gm_base (cast `/Game/Blueprints/BP_GM_Base` (`GameplayStatics.GetGameMode`)))
    (bind _quest_manager (`/Game/Blueprints/BP_GM_Base.Quest Manager` _asbp_gm_base))
    (`/Engine/EditorBlueprintResources/StandardMacros.IsValid` _quest_manager
      (:`Is Valid`
        (`QuestManager.setActiveQuest` _quest_manager (- (`QuestManager.ActiveQuestId` _quest_manager) 1))))))

(event `self.StopAim`
  (bind _mainwidget (`self.MainWidget`))
  ;[1 1 1] Aiming UI
  (`parent.StopAim`)
  (`Widget.SetVisibility` (`/Game/UI/Widget_HUD.ReticleWide` _mainwidget) "Visible")
  (`Widget.SetVisibility` (`/Game/UI/Widget_HUD.Reticle` _mainwidget) "Hidden"))

(event `self.Damage`
  (params (dmg :type "Float (single-precision)"))
  ;[1 1 1] Damage Sounds
  (`parent.Damage` dmg)
  (if (== (`KismetMathLibrary.RandomIntegerInRange` 0 1) 0)
    (`GameplayStatics.PlaySoundAtLocation` "/Game/Sounds/Mech/S_Hit1.S_Hit1" (`self.K2_GetActorLocation`) (struct) 1.0 1.0 0.0 null null null)
    (else
      (`GameplayStatics.PlaySoundAtLocation` "/Game/Sounds/Mech/S_Hit2.S_Hit2" (`self.K2_GetActorLocation`) (struct) 1.0 1.0 0.0 null null null))))

(event `Key|Two`
  (params (Key :type "Key Structure"))
  ;[1 1 1] Quest Switching
  (:`Pressed`
    (bind _asbp_gm_base (cast `/Game/Blueprints/BP_GM_Base` (`GameplayStatics.GetGameMode`)))
    (bind _quest_manager (`/Game/Blueprints/BP_GM_Base.Quest Manager` _asbp_gm_base))
    (`/Engine/EditorBlueprintResources/StandardMacros.IsValid` _quest_manager
      (:`Is Valid`
        (`QuestManager.setActiveQuest` _quest_manager (+ (`QuestManager.ActiveQuestId` _quest_manager) 1))))))

(event `self.Mount`
  (bind (_defaultcamtrans_location _defaultcamtrans_rotation) (`KismetMathLibrary.BreakTransform` (`self.DefaultCamTrans`)))
  (bind (_returnvalue_location _returnvalue_rotation) (`KismetMathLibrary.BreakTransform` (`SceneComponent.GetRelativeTransform` (`self.RightCamPos`))))
  (bind (_returnvalue_location_2 _returnvalue_rotation_2) (`KismetMathLibrary.BreakTransform` (`SceneComponent.GetRelativeTransform` (`self.LeftCamPos`))))
  (bind _relativelocation (`SceneComponent.RelativeLocation` (`self.FollowCamera`)))
  ;[1 1 1] Mount Animation Stuff
  (if (<= (`KismetMathLibrary.VSizeSquared` (- _relativelocation (`SceneComponent.RelativeLocation` (`self.RightCamPos`)))) (`KismetMathLibrary.VSizeSquared` (- _relativelocation (`SceneComponent.RelativeLocation` (`self.LeftCamPos`)))))
    (`KismetSystemLibrary.MoveComponentTo` (`self.FollowCamera`) _returnvalue_location _returnvalue_rotation true false 2.0)
    (else
      (`KismetSystemLibrary.MoveComponentTo` (`self.FollowCamera`) _returnvalue_location_2 _returnvalue_rotation_2 true false 2.0)))
  (`KismetSystemLibrary.MoveComponentTo` (`self.FollowCamera`) _defaultcamtrans_location _defaultcamtrans_rotation false true 2.0)
  (`self.SetUIVisability` true))

(event `self.Dismount`
  (`self.SetUIVisability` false)
  (`parent.Dismount`))

(event `SetUIVisability`
  (params (isVisable :type Boolean))
  (if isVisable
    (`Widget.SetVisibility` (`self.MainWidget`) "Visible")
    (`Widget.SetVisibility` (`self.QuestWidget`) "Visible")
    (else
      (`Widget.SetVisibility` (`self.MainWidget`) "Hidden")
      (`Widget.SetVisibility` (`self.QuestWidget`) "Hidden"))))

(fn `UserConstructionScript`)