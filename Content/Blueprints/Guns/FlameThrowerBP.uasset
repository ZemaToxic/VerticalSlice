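; Flamethrower gun Blueprint that adds start, idle and end audio to the shooting behavior of its parent class.
; Shoot calls the parent, then plays the Salamander start sound and runs a fast looping timer if Shooting is set.
; The timer polls until the start sound component is no longer valid, then switches to the idle sound.
; StopShoot cuts the active sound, plays the end sound, clears the timer and calls the parent.
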(event `self.Shoot`
  (`parent.Shoot`)
  (if (`self.Shooting`)
    (bind _returnvalue (`GameplayStatics.CreateSound2D` "/Game/Sounds/Mech/S_SalamanderStart.S_SalamanderStart" 1.0 1.0 0.0 null))
    (bind _output_get (set `self.SoundStart` _returnvalue))
    (`AudioComponent.Play` _output_get 0.0)
    (bind _returnvalue_2 (`KismetSystemLibrary.K2_SetTimerDelegate` (delegate `CheckSound`) 0.01 true))
    (set `self.TimerCheck` _returnvalue_2)))

(event `CheckSound`
  (`/Engine/EditorBlueprintResources/StandardMacros.IsValid` (`self.SoundStart`)
    (:`Is Not Valid`
      (bind _returnvalue (`GameplayStatics.CreateSound2D` "/Game/Sounds/Mech/S_SalamanderIdle.S_SalamanderIdle" 1.0 1.0 0.0 null))
      (bind _output_get (set `self.SoundLoop` _returnvalue))
      (`AudioComponent.Play` _output_get 0.0)
      (`KismetSystemLibrary.K2_ClearAndInvalidateTimerHandle` (`self.TimerCheck`)))))

(event `self.StopShoot`
  (bind _soundstart (`self.SoundStart`))
  (bind _soundloop (`self.SoundLoop`))
  (if (`self.Shooting`)
    (`/Engine/EditorBlueprintResources/StandardMacros.IsValid` _soundstart
      (:`Is Valid`
        (`AudioComponent.Stop` _soundstart))
      (:`Is Not Valid`
        (`/Engine/EditorBlueprintResources/StandardMacros.IsValid` _soundloop
          (:`Is Valid`
            (if (`AudioComponent.IsPlaying` _soundloop)
              (`AudioComponent.Stop` _soundloop)))
          (:`Is Not Valid`
            _))))
    (`GameplayStatics.PlaySound2D` "/Game/Sounds/Mech/S_SalamanderEnd.S_SalamanderEnd" 1.0 1.0 0.0 null null)
    (`KismetSystemLibrary.K2_ClearAndInvalidateTimerHandle` (`self.TimerCheck`))
    (`parent.StopShoot`)))

(fn `UserConstructionScript`)