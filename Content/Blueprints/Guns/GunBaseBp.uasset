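; Base gun Blueprint that adds shot feedback to the parent's raycast shooting.
; ShootRaycasts calls the parent, then, if the player pawn is MechBoi2, plays two shot animations on its main widget.
; It spawns trails from the shot start toward each hit and shot end, timing their lifetime from distance over trail speed, plus bullet-hole decals at hits.
; An older beam-particle trail remains as unconnected nodes.
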(event `self.ReceiveTick`
  (params (DeltaSeconds :type "Float (single-precision)")))

(event `self.ShootRaycasts`
  (bind _trailspeed (`self.TrailSpeed`))
  (bind _shotstart (`self.shotStart`))
  (bind _trailspeed_2 (`self.TrailSpeed`))
  (`parent.ShootRaycasts`)
  (bind _asmech_boi_2 (cast `/Game/Blueprints/Player/MechBoi2` (`GameplayStatics.GetPlayerPawn` 0)))
  ;[1 1 1] Add trail here
  (`|ExecutionSequence`
    (:`then_0`
      (bind _mainwidget (`/Game/Blueprints/Player/MechBoi2.MainWidget` _asmech_boi_2))
      (`UserWidget.PlayAnimation` _mainwidget (`/Game/UI/Widget_HUD.Shot` _mainwidget) 0.0 1 "Forward" 1.0 false))
    (:`then_1`
      (`UserWidget.PlayAnimation` _mainwidget (`/Game/UI/Widget_HUD.Shot_0` _mainwidget) 0.0 1 "Forward" 1.0 false))
    (:`then_2`
      ;[1 1 1] Projectile effects
      (for _array_element (`self.hitResults`)
        (`|SpawnActorFromClass` "/Game/Effects/BP/BP_Trail.BP_Trail_C" (`KismetMathLibrary.MakeTransform` _shotstart (`KismetMathLibrary.FindLookAtRotation` _shotstart (`.ImpactPoint` (`GameplayStatics.BreakHitResult` _array_element)))) "Undefined" "OverrideRootScale" null (/ (`KismetMathLibrary.Abs` (`KismetMathLibrary.VSize` (- (`.ImpactPoint` (`GameplayStatics.BreakHitResult` _array_element)) _shotstart))) _trailspeed_2) _trailspeed_2 null)
        (`|SpawnActorFromClass` "/Game/Effects/BP/DecalActor_BulletHoles.DecalActor_BulletHoles_C" (`KismetMathLibrary.MakeTransform` (`.ImpactPoint` (`GameplayStatics.BreakHitResult` _array_element)) (`KismetMathLibrary.MakeRotationFromAxes` (`.Normal` (`GameplayStatics.BreakHitResult` _array_element)))) "Undefined" "OverrideRootScale" null null))
      (for _array_element_2 (`self.shotEnd`)
        (`|SpawnActorFromClass` "/Game/Effects/BP/BP_Trail.BP_Trail_C" (`KismetMathLibrary.MakeTransform` _shotstart (`KismetMathLibrary.FindLookAtRotation` _shotstart _array_element_2)) "Undefined" "OverrideRootScale" null (/ (`KismetMathLibrary.Abs` (`KismetMathLibrary.VSize` (- _array_element_2 _shotstart))) _trailspeed) _trailspeed null)))))

(fn `UserConstructionScript`)