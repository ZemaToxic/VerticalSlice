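; Workshop station actor that opens the workshop menu when its overlapping InteractableVolume, found on BeginPlay, is activated.
; Tick polls that volume, then restocks via the game mode, disables pawn input, shows the workshop widget, repositions the player's mech facing the station and destroys all drops.
; Escape or Interact calls the widget's Exit, with a short delay before clearing the open flag to prevent immediate reopening.
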(event `self.ReceiveBeginPlay`
  (bind _asinteractable_volume (cast `InteractableVolume` (`|GetArrayItem` (`PrimitiveComponent.GetOverlappingActors` (`self.Box`) "/Script/VerticalSlice.InteractableVolume")))
    (:`then`
      (set `self.InteractActor` _asinteractable_volume))
    (:`CastFailed`
      _))
  (`KismetSystemLibrary.Delay` 0.2)
  (`self.EnableInput` (`GameplayStatics.GetPlayerController` 0)))

(event `self.ReceiveTick`
  (params (DeltaSeconds :type "Float (single-precision)"))
  (bind _returnvalue (`GameplayStatics.GetPlayerController` 0))
  (bind _returnvalue_2 (`GameplayStatics.GetPlayerPawn` 0))
  (bind _returnvalue_3 (`self.K2_GetActorLocation`))
  (bind _returnvalue_4 (+ (+ _returnvalue_3 (* (`SceneComponent.GetForwardVector` (`self.Arrow`)) 1000.0)) (* (`self.GetActorUpVector`) 100.0)))
  (bind (_returnvalue_roll _returnvalue_pitch _returnvalue_yaw) (`KismetMathLibrary.BreakRotator` (`KismetMathLibrary.FindLookAtRotation` _returnvalue_4 _returnvalue_3)))
  ;[1 1 1] Make sure workshop is not open
  (if (and (`InteractableVolume.GetActivated` (`self.InteractActor`)) (not (`self.WorkshopOpen`)))
    (bind _asbp_gm_base (cast `/Game/Blueprints/BP_GM_Base` (`GameplayStatics.GetGameMode`)))
    (`/Game/Blueprints/BP_GM_Base.Restock` _asbp_gm_base)
    (bind _output_get (set `self.PlayerPawn` _returnvalue_2))
    (`self.DisableInput` _output_get _returnvalue)
    (set `self.PlayerController` _returnvalue)
    (bind _asthird_person_character (cast `/Game/Blueprints/Player/ThirdPersonCharacter` _returnvalue_2))
    (set `/Game/Blueprints/Player/ThirdPersonCharacter.InWorkshop` true _asthird_person_character)
    (set `PlayerController.bShowMouseCursor` true (`self.PlayerController`))
    (bind _returnvalue_5 (`|CreateWidget` "/Game/UI/Widget_Workshop3.Widget_Workshop3_C" (`self.PlayerController`)))
    (bind _output_get_2 (set `self.Workshop` _returnvalue_5))
    (`WidgetBlueprintLibrary.SetInputMode_GameAndUIEx` (`self.PlayerController`) _output_get_2)
    (`UserWidget.AddToViewport` _output_get_2 0)
    (set `self.WorkshopOpen` true)
    (bind _asthird_person_character_2 (cast `/Game/Blueprints/Player/ThirdPersonCharacter` (`self.PlayerPawn`)))
    (bind _playermech (`VerticalSliceCharacter.PlayerMech` _asthird_person_character_2))
    (bind _asmech_boi_2 (cast `/Game/Blueprints/Player/MechBoi2` _playermech))
    (`/Game/Blueprints/Player/MechBoi2.SetQuestVisibility` _asmech_boi_2 false)
    (`self.K2_SetActorLocationAndRotation` _playermech _returnvalue_4 (`KismetMathLibrary.MakeRotator` 0.0 0.0 _returnvalue_yaw) false false)
    (`self.DestroyDrops`)
    (`GameplayStatics.PlaySound2D` "/Game/Sounds/UI/S_Save.S_Save" 1.0 1.0 0.0 null null)))

(event `InputAction|Pause`
  (params (Key :type "Key Structure")))

(event `Key|Escape` :consume false
  (params (Key :type "Key Structure"))
  (:`Pressed`
    (if (`self.WorkshopOpen`) :!label _label
      (`self.CloseWorkshop`)
      (`KismetSystemLibrary.Delay` 0.1) ; Prevent the player from reopening immediately
      (set `self.WorkshopOpen` false))))

(event `Key|H`
  (params (Key :type "Key Structure")))

(event `InputAction|Interact` :consume false
  (params (Key :type "Key Structure"))
  (:`Pressed`
    (goto _label)))

(fn `CloseWorkshop`
  (bind _workshop (`self.Workshop`))
  (set `/Game/UI/Widget_Workshop3.PlayerPawn` (`self.PlayerPawn`) _workshop)
  (`/Game/UI/Widget_Workshop3.Exit` _workshop))

(fn `DestroyDrops`
  (bind _outactors (`GameplayStatics.GetAllActorsOfClass` "/Script/VerticalSlice.DropsBase"))
  (for _array_element _outactors
    (`self.K2_DestroyActor` _array_element)))

(fn `UserConstructionScript`)