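; Base game mode for the mech game that runs quests, restocks the player's mech, shows part-drop popups and opens the pause menu.
; BeginPlay spawns a QuestManager, loads QuestA1.1 and indexes interactable volumes by ID.
; Looping timers update objective locations and values, inferring kills from falling monster counts, driving the waypoint widget and advancing stages until completion.
; Monsters spawn at EQS-selected locations, with debug spheres and a test spawn input.
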(event `self.ReceiveBeginPlay`
  (bind _returnvalue (`GameplayStatics.GetPlayerController` 0))
  (bind _outactors (`GameplayStatics.GetAllActorsOfClass` "/Game/Blueprints/Player/MechBoi2.MechBoi2_C"))
  (bind _output (`|GetArrayItem` _outactors))
  (`/Engine/EditorBlueprintResources/StandardMacros.IsValid` _output
    (:`Is Valid`
      (set `self.MechRef` _output)
      (`WidgetBlueprintLibrary.SetInputMode_GameOnly` _returnvalue)
      (set `PlayerController.bShowMouseCursor` false _returnvalue)
      ;[1 1 1] Quest Stuff
      (bind _returnvalue_2 (`|SpawnActorFromClass` "/Script/QuestPlugin.QuestManager" (`KismetMathLibrary.MakeTransform` (0.0 0.0 0.0)) "Undefined" "OverrideRootScale" null null))
      (set `self.Quest Manager` _returnvalue_2)
      (bind _success (`QuestManager.LoadQuest` (`self.Quest Manager`) "QuestA1.1"))
      (if _success
        (`self.Start quest checking`)
        (bind _outactors_2 (`GameplayStatics.GetAllActorsOfClass` "/Script/VerticalSlice.InteractableVolume"))
        (for _array_element _outactors_2
          (bind _returnvalue_3 (- (`InteractableVolume.id` _array_element) 2))
          (if (>= _returnvalue_3 0)
            (`KismetArrayLibrary.Array_Set` (`self.Interactable objects`) _returnvalue_3 _array_element true)))
        (`self.EnableInput` (`GameplayStatics.GetPlayerController` 0))))))

(event `Restock`
  (bind _mechref (`self.MechRef`))
  (`Mech.giveAmmo` _mechref true 0)
  (`Mech.giveHealth` _mechref true 0))

(event `self.AddParts`
  (params (_dropType :type "MonsterDrops Enum" :default "NOTHING") (_amount :type Integer))
  (`parent.AddParts` _dropType _amount)
  (bind _returnvalue (`|CreateWidget` "/Game/UI/Widget_Drops.Widget_Drops_C" (`GameplayStatics.GetPlayerController` 0) (`|GetEnumeratorNameAsString` _dropType) _amount))
  (`UserWidget.AddToViewport` _returnvalue 0))

(event `Stop Quest Checking`
  ;[1 1 1] More quest stuff
  (`KismetSystemLibrary.K2_PauseTimerHandle` (`self.LocationUpdate`))
  (`KismetSystemLibrary.K2_PauseTimerHandle` (`self.Value Update`)))

(event `Start Quest Checking`
  (bind _locationupdate (`self.LocationUpdate`))
  (bind _value_update (`self.Value Update`))
  ;[1 1 1] More quest stuff
  (if (`KismetSystemLibrary.K2_IsValidTimerHandle` _locationupdate)
    (`KismetSystemLibrary.K2_UnPauseTimerHandle` _locationupdate)
    (else
      (bind _returnvalue (`KismetSystemLibrary.K2_SetTimerDelegate` (delegate `UpdateLoc`) 0.1 true))
      (set `self.LocationUpdate` _returnvalue)
      (if (`KismetSystemLibrary.K2_IsValidTimerHandle` _value_update)
        (`KismetSystemLibrary.K2_UnPauseTimerHandle` _value_update)
        (else
          (bind _returnvalue_2 (`KismetSystemLibrary.K2_SetTimerDelegate` (delegate `Update Values`) 0.1 true))
          (set `self.Value Update` _returnvalue_2))))))

(event `UpdateLoc`
  (bind _activequest (`QuestManager.ActiveQuest` (`self.Quest Manager`)))
  ;[1 1 1] More quest stuff
  (`/Engine/EditorBlueprintResources/StandardMacros.IsValid` _activequest
    (:`Is Valid`
      (`ActiveQuest.updateAllLocations` _activequest (`self.K2_GetActorLocation` (`GameplayStatics.GetPlayerPawn` 0))))))

(event `Update Values`
  (bind _currentenemycount (`self.CurrentEnemyCount`))
  (bind _previousenemycount (`self.PreviousEnemyCount`))
  (bind _activequest (`QuestManager.ActiveQuest` (`self.Quest Manager`)))
  (bind _quest (`ActiveQuest.Quest` (`QuestManager.ActiveQuest` (`self.Quest Manager`))))
  (bind _returnvalue (`KismetArrayLibrary.Array_Length` _quest))
  ;[1 1 1] More quest stuff
  (bind _quest_complete (`self.CheckComplete`))
  (if _quest_complete
    (`/QuestPlugin/QuestUI.TurnOffDisplay` (`/Game/Blueprints/Player/MechBoi2.QuestWidget` (`self.MechRef`)))
    (`self.Stop Quest Checking`)
    ;;[1 0 0] DEBUG
    (`KismetSystemLibrary.PrintString` "Quest Complete")
    (else
      (bind _outactors (`GameplayStatics.GetAllActorsOfClass` "/Game/Blueprints/Monsters/BP_MonsterBase.BP_MonsterBase_C"))
      (set `self.CurrentEnemyCount` (`KismetArrayLibrary.Array_Length` _outactors))
      (if (> _returnvalue 0)
        (set `self.QuestHasLoc` false)
        (for _index (range _returnvalue)
          (bind (_output_questname _output_questdescription _output_objectivename _output_typeint _output_usesvalue _output_objectivecompletevalue _output_useslocation _output_location) (break `QuestStruct` (`|GetArrayItem` _quest _index)))
          (switch `int` _output_typeint
            (:`Default`
              (if (`InteractableVolume.activated` (`|GetArrayItem` (`self.Interactable objects`) (- _output_typeint 2)))
                (`ActiveQuest.addToValue` _activequest _index 1.0)))
            (:`0`
              (set `/QuestPlugin/QuestUI.TrackedLoc` _output_location (`/Game/Blueprints/Player/MechBoi2.QuestWidget` (`self.MechRef`)))
              (set `self.QuestHasLoc` true))
            (:`1`
              (if (< _currentenemycount _previousenemycount)
                (`ActiveQuest.addToValue` _activequest _index (`KismetMathLibrary.Conv_IntToDouble` (- _previousenemycount _currentenemycount)))))))
        (set `self.PreviousEnemyCount` (`self.CurrentEnemyCount`))
        (`/QuestPlugin/QuestUI.Change WaypointState` (`/Game/Blueprints/Player/MechBoi2.QuestWidget` (`self.MechRef`)) (`self.QuestHasLoc`))))))

(event `InputAction|Pause`
  (params (Key :type "Key Structure"))
  (bind _returnvalue (`GameplayStatics.GetPlayerController` 0))
  ;[1 1 1] Pause
  (:`Pressed`
    (bind _returnvalue_2 (`|CreateWidget` "/Game/UI/Widget_Pause.Widget_Pause_C" _returnvalue))
    (`UserWidget.AddToViewport` _returnvalue_2 0)
    (set `PlayerController.bShowMouseCursor` true _returnvalue)
    (`WidgetBlueprintLibrary.SetInputMode_UIOnlyEx` _returnvalue _returnvalue_2)))

(event `InputAction|Spawn`
  (params (Key :type "Key Structure"))
  (:`Pressed`
    (`self.SpawnMonstersAtLocation` "TEST" 5 "/Game/Blueprints/Monsters/BP_MonsterB.BP_MonsterB_C" "/Game/AI/BT_MonsterB.BT_MonsterB")))

(event `self.SpawnMonsters`
  (bind _returnvalue (`EnvQueryManager.RunEQSQuery` "/Game/AI/EQS/EQS_FindSpawnLoc.EQS_FindSpawnLoc" self "RandomBest25Pct"))
  (add `EnvQueryInstanceBlueprintWrapper.OnQueryFinishedEvent` _returnvalue (delegate `OnQueryFinishedEvent_Event_0`)))

(event `OnQueryFinishedEvent_Event_0`
  (params (QueryInstance :type "EnvQueryInstanceBlueprintWrapper Object Reference") (QueryStatus :type "EEnvQueryStatus Enum" :default "Processing"))
  (switch `EEnvQueryStatus` QueryStatus
    (:`Success`
      (bind _resultlocations (`EnvQueryInstanceBlueprintWrapper.GetQueryResultsAsLocations` QueryInstance))
      (for _array_element _resultlocations
        (`KismetSystemLibrary.DrawDebugSphere` _array_element 64.0 12 (struct :`R` 1.0 :`G` 0.737436 :`A` 1.0) 3.0 2.0)
        (`AIBlueprintHelperLibrary.SpawnAIFromClass` (`self.MonsterToSpawn`) (`self.BT`) _array_element)))))

(fn `CheckComplete`
  (returns (`Quest Complete` :type Boolean))
  (bind _activequest (`QuestManager.ActiveQuest` (`self.Quest Manager`)))
  (bind _complete (`ActiveQuest.checkAllObjectivesComplete` _activequest))
  (if _complete
    (bind _success (`ActiveQuest.loadNextStage` _activequest))
    (if _success
      (for _array_element (`ActiveQuest.Quest` _activequest)
        (if (>= (`.typeInt` (break `QuestStruct` _array_element)) 2)
          (set `InteractableVolume.activated` false (`|GetArrayItem` (`self.Interactable objects`) (- (`.typeInt` (break `QuestStruct` _array_element)) 2)))
          (return (not _success))))
      (else
        (return (not _success))))
    (else
      (return false))))

(fn `UserConstructionScript`)