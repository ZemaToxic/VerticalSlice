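; Boss energy projectile that bursts into an expanding blast when it stops or its lifetime timer runs out.
; Stopping also disables sphere collision, plays impact particles and sound, and clears the timer.
; A one-shot guarded timeline scales the visual sphere and Explosion overlap volume while fading material opacity, then destroys the actor.
; Explosion overlaps damage MechBoi2 actors and kill ThirdPersonCharacters outright.
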(event `self.ReceiveBeginPlay`
  (bind _returnvalue (`KismetSystemLibrary.K2_SetTimerDelegate` (delegate `DestroyAfterXSeconds`) (`self.DestroyAfterTime`))))

(event `Print Location`
  ;[1 0 0] Debugging
  (`KismetSystemLibrary.PrintString` (`KismetStringLibrary.Conv_VectorToString` (`self.K2_GetActorLocation`))))

(event `DestroyAfterXSeconds`
  (`self.StartExplosion`))

(event `self.ProjectileMovement.OnProjectileStop`
  (params (ImpactResult :type "HitResult Structure (by ref)"))
  ;[1 1 1] Projectile Stop
  (`PrimitiveComponent.SetCollisionResponseToAllChannels` (`self.Sphere`) "ECR_Ignore")
  (`NiagaraFunctionLibrary.SpawnSystemAtLocation` "/Game/Effects/Niagra/P_BossEnergyImpact.P_BossEnergyImpact" ImpactResult_Location)
  (`GameplayStatics.PlaySoundAtLocation` "/Game/Sounds/Monster/S_BossEnergyExplosion.S_BossEnergyExplosion" ImpactResult_Location (struct) 1.0 1.0 0.0 null null null)
  (`KismetSystemLibrary.K2_ClearAndInvalidateTimerHandle` (stale `self.ReceiveBeginPlay` _returnvalue))
  (`self.StartExplosion`))

(event `self.Explosion.OnComponentBeginOverlap`
  (params (OverlappedComponent :type "PrimitiveComponent Object Reference") (OtherActor :type "Actor Object Reference") (OtherComp :type "PrimitiveComponent Object Reference") (OtherBodyIndex :type Integer) (bFromSweep :type Boolean) (SweepResult :type "HitResult Structure (by ref)"))
  ;[1 1 1] Check for overlap
  (bind _asmech_boi_2 (cast `/Game/Blueprints/Player/MechBoi2` OtherActor)
    (:`then`
      (`Mech.Damage` _asmech_boi_2 (`self.Damage`) (0.0 0.0 0.0)))
    (:`CastFailed`
      (bind _asthird_person_character (cast `/Game/Blueprints/Player/ThirdPersonCharacter` OtherActor))
      (`/Game/Blueprints/Player/ThirdPersonCharacter.Kill` _asthird_person_character))))

(event `self.StartExplosion`
  ;[1 1 1] Start Explosion
  (if (not (`self.IsExploding`))
    (`MovementComponent.StopMovementImmediately` (`self.ProjectileMovement`))
    (set `self.IsExploding` true)
    (bind (_direction _lerp0_1 _opacity) (`Timeline|Timeline_0`)
      (:`Update`
        (bind _returnvalue (* (1.0 1.0 1.0) (`KismetMathLibrary.Lerp` (`self.ExplosionBeginRadius`) (`self.ExplosionEndRadius`) _lerp0_1)))
        (`SceneComponent.SetWorldScale3D` (`self.Sphere`) _returnvalue)
        (`SceneComponent.SetWorldScale3D` (`self.Explosion`) _returnvalue)
        (`MeshComponent.SetScalarParameterValueOnMaterials` (`self.Sphere`) "Energy_Opacity" (`KismetMathLibrary.Lerp` 0.05 0.0 _opacity)))
      (:`Finished`
        (`self.K2_DestroyActor`)))))

(fn `UserConstructionScript`)