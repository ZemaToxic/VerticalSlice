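; BP_MonsterB is a monster Blueprint whose AI perception tracks whether it senses the player.
; Target perception updates for the player pawn set the CanSeePlayer blackboard key and a FacePlayer flag.
; While that flag is set, Tick smoothly turns the monster's yaw toward the player character.
; CompleteSenses, which would also write investigation state and stimulus location, is only called from unconnected logic, so it never runs.
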(event `self.ReceiveBeginPlay`
  (`parent.ReceiveBeginPlay`))

(event `self.ReceiveTick`
  (params (DeltaSeconds :type "Float (single-precision)"))
  (`parent.ReceiveTick` DeltaSeconds)
  (set `self.Delta` DeltaSeconds)
  (`self.RotateToPlayer`))

(event `self.AIPerception.OnTargetPerceptionUpdated`
  (params (Actor :type "Actor Object Reference") (Stimulus :type "AIStimulus Structure"))
  (bind (_age _expirationage _strength _stimuluslocation _receiverlocation _tag _bsuccessfullysensed) (break `AIStimulus` Stimulus))
  (if (== (`GameplayStatics.GetPlayerPawn` 0) Actor)
    (`BlackboardComponent.SetValueAsBool` (`AIBlueprintHelperLibrary.GetBlackboard` null) "CanSeePlayer" _bsuccessfullysensed)
    (set `self.FacePlayer` _bsuccessfullysensed)))

(event `self.AIPerception.OnPerceptionUpdated`
  (params (UpdatedActors :type "Array of Actor Object Reference (by ref)")))

(fn `CompleteSenses`
  (params (Array :type "Array of AIStimulus Structure"))
  (bind (_localsense_age _localsense_expirationage _localsense_strength _localsense_stimuluslocation _localsense_receiverlocation _localsense_tag _localsense_bsuccessfullysensed) (break `AIStimulus` (`self.LocalSense`)))
  (for (_array_element _array_index) Array
    (set `self.LocalSense` _array_element)
    (switch `int` _array_index
      (:`0`
        (`BlackboardComponent.SetValueAsBool` (`AIBlueprintHelperLibrary.GetBlackboard` null) "CanSeePlayer" _localsense_bsuccessfullysensed)
        (set `self.FacePlayer` _localsense_bsuccessfullysensed))
      (:`1`
        (if _localsense_bsuccessfullysensed
          (`BlackboardComponent.SetValueAsBool` (`AIBlueprintHelperLibrary.GetBlackboard` null) "IsInvestigating" _localsense_bsuccessfullysensed :!label _label)
          (`BlackboardComponent.SetValueAsVector` (`AIBlueprintHelperLibrary.GetBlackboard` null) "TargetLocation" _localsense_stimuluslocation)))
      (:`2`
        (if _localsense_bsuccessfullysensed
          (goto _label))))))

(fn `RotateToPlayer`
  (bind _returnvalue (`GameplayStatics.GetPlayerCharacter` 0))
  (bind (_returnvalue_roll _returnvalue_pitch _returnvalue_yaw) (`KismetMathLibrary.BreakRotator` (`KismetMathLibrary.RInterpTo` (`self.K2_GetActorRotation`) (`KismetMathLibrary.FindLookAtRotation` (`self.K2_GetActorLocation`) (`self.K2_GetActorLocation` _returnvalue)) (`self.Delta`) 2.0)))
  (`/Engine/EditorBlueprintResources/StandardMacros.IsValid` _returnvalue
    (:`Is Valid`
      (if (`self.FacePlayer`)
        (`self.K2_SetActorRotation` (`KismetMathLibrary.MakeRotator` 0.0 0.0 _returnvalue_yaw))))))

(fn `UserConstructionScript`
  (`parent.UserConstructionScript`))