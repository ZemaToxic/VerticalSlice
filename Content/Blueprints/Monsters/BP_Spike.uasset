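; BP_Spike is a short-lived monster spike that harms players on contact and removes itself.
; Capsule overlap damages a Mech at the spike's location or kills a ThirdPersonCharacter outright, destroying the spike in both cases.
; Other overlaps also destroy it, except its owner, drops and other monsters, which it ignores.
; Any capsule hit destroys it, and a timer started on BeginPlay cleans up spikes that strike nothing.
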(event `self.ReceiveBeginPlay`
  (`KismetSystemLibrary.K2_SetTimerDelegate` (delegate `Delete`) 5.0))

(event `Delete`
  (`self.K2_DestroyActor`))

(event `self.Capsule.OnComponentBeginOverlap`
  (params (OverlappedComponent :type "PrimitiveComponent Object Reference") (OtherActor :type "Actor Object Reference") (OtherComp :type "PrimitiveComponent Object Reference") (OtherBodyIndex :type Integer) (bFromSweep :type Boolean) (SweepResult :type "HitResult Structure (by ref)"))
  (bind _asmech (cast `Mech` OtherActor)
    (:`then`
      (`Mech.Damage` _asmech (`self.Damage`) (`SceneComponent.K2_GetComponentLocation` OverlappedComponent))
      (`self.K2_DestroyActor`))
    (:`CastFailed`
      (bind _asthird_person_character (cast `/Game/Blueprints/Player/ThirdPersonCharacter` OtherActor)
        (:`then`
          (`self.K2_DestroyActor`)
          (`/Game/Blueprints/Player/ThirdPersonCharacter.Kill` _asthird_person_character))
        (:`CastFailed`
          (if (not (== (`self.GetOwner`) OtherActor))
            (cast `/Game/Blueprints/Drops/BP_DropsBase` OtherActor ; Ignore Drops
              (:`CastFailed`
                (cast `/Game/Blueprints/Monsters/BP_MonsterBase` OtherActor ; Ignore Other Monsters
                  (:`CastFailed`
                    (`self.K2_DestroyActor`)))))))))))

(event `self.Capsule.OnComponentHit`
  (params (HitComponent :type "PrimitiveComponent Object Reference") (OtherActor :type "Actor Object Reference") (OtherComp :type "PrimitiveComponent Object Reference") (NormalImpulse :type "Vector Structure") (Hit :type "HitResult Structure (by ref)"))
  (`self.K2_DestroyActor`))

(fn `UserConstructionScript`)