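; BP_RockyGroundWave is a monster ground attack that advances forward as timed rows of rocky eruptions.
; Each actor spawns one row of BP_RockySingleEruption across its right vector, sized by its Widths entry and centered for odd or even counts.
; It chains the wave by spawning a successor a set distance ahead with an incremented iteration, then destroys itself shortly after, until the Widths array is exhausted.
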(event `self.ReceiveBeginPlay`
  (set `self.MaxIterations` (`KismetArrayLibrary.Array_Length` (`self.Widths`)))
  (`self.CheckSpawnRequired`)
  (`self.SpawnFX`)
  (`KismetSystemLibrary.K2_SetTimer` null "DestroySelf" (+ (`self.DelayBetweenExplosions`) 0.2)))

(event `DestroySelf`
  (`self.K2_DestroyActor`))

(event `CheckSpawnRequired`
  (if (< (`self.CurrentIteration`) (- (`self.MaxIterations`) 1))
    (`KismetSystemLibrary.K2_SetTimer` null "SpawnNext" (`self.DelayBetweenExplosions`))))

(event `SpawnNext`
  (`|SpawnActorFromClass` "BP_RockyGroundWave_C" (`KismetMathLibrary.MakeTransform` (+ (* (`self.GetActorForwardVector`) (`self.DistanceBetweenWaves`)) (`self.K2_GetActorLocation`)) (`self.K2_GetActorRotation`)) "Undefined" "OverrideRootScale" null (+ (`self.CurrentIteration`) 1) null))

(fn `SpawnFX`
  (bind _returnvalue (/ (`|GetArrayItem` (`self.Widths`) (`self.CurrentIteration`)) 2))
  (if (== (mod (`|GetArrayItem` (`self.Widths`) (`self.CurrentIteration`)) 2) 0)
    (`|ExecutionSequence`
      (:`then_0`
        (for _index (range (/ (`|GetArrayItem` (`self.Widths`) (`self.CurrentIteration`)) 2))
          (`|SpawnActorFromClass` "/Game/Blueprints/Monsters/BP_RockySingleEruption.BP_RockySingleEruption_C" (`KismetMathLibrary.MakeTransform` (+ (`self.K2_GetActorLocation`) (* (`self.GetActorRightVector`) (+ (* _index (* 2 (`self.CapsuleRadius`))) (`self.CapsuleRadius`)))) (`self.K2_GetActorRotation`)) "Undefined" "OverrideRootScale" null (`self.EruptionDelay`) null)))
      (:`then_1`
        (for _index_2 (range (/ (`|GetArrayItem` (`self.Widths`) (`self.CurrentIteration`)) 2))
          (`|SpawnActorFromClass` "/Game/Blueprints/Monsters/BP_RockySingleEruption.BP_RockySingleEruption_C" (`KismetMathLibrary.MakeTransform` (+ (`self.K2_GetActorLocation`) (* (* (`self.GetActorRightVector`) -1.0) (+ (* _index_2 (* 2 (`self.CapsuleRadius`))) (`self.CapsuleRadius`)))) (`self.K2_GetActorRotation`)) "Undefined" "OverrideRootScale" null (`self.EruptionDelay`) null))))
    (else
      (for _index_3 (range (* _returnvalue -1) (+ _returnvalue 1))
        (`|SpawnActorFromClass` "/Game/Blueprints/Monsters/BP_RockySingleEruption.BP_RockySingleEruption_C" (`KismetMathLibrary.MakeTransform` (+ (`self.K2_GetActorLocation`) (* (`self.GetActorRightVector`) (* _index_3 (* (`self.CapsuleRadius`) 2.0)))) (`self.K2_GetActorRotation`)) "Undefined" "OverrideRootScale" null (`self.EruptionDelay`) null)))))

(fn `UserConstructionScript`)