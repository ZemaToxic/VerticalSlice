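; Single rock eruption hazard for a boss, which hurts the player's mech or kills an on-foot character.
; On BeginPlay it optionally plays a slam effect as a delayed warning, then spawns the rock burst and starts polling capsule overlaps on a fast looping timer.
; The first mech found takes damage, otherwise a third-person character is killed, and either hit disarms the eruption.
; The actor destroys itself after its active time.
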(event `self.ReceiveBeginPlay`
  (if (> (`self.EruptionDelay`) 0.0)
    (`NiagaraFunctionLibrary.SpawnSystemAtLocation` "/Game/Effects/Niagra/P_RockySlam.P_RockySlam" (`self.K2_GetActorLocation`) (`self.K2_GetActorRotation`))
    (`KismetSystemLibrary.Delay` (`self.EruptionDelay`)))
  (`NiagaraFunctionLibrary.SpawnSystemAtLocation` "/Game/Effects/Niagra/P_BossRocks.P_BossRocks" (`self.K2_GetActorLocation`) (`self.K2_GetActorRotation`))
  (`KismetSystemLibrary.K2_SetTimer` null "Deactivate" (`self.ActiveTime`))
  (set `self.CanHit` true)
  (`ActorComponent.Activate` (`self.Capsule`) false)
  (bind _returnvalue (`KismetSystemLibrary.K2_SetTimer` null "CheckHit_0" 0.01 true)))

(event `Deactivate`
  (`KismetSystemLibrary.K2_ClearAndInvalidateTimerHandle` (stale `self.ReceiveBeginPlay` _returnvalue))
  (`self.K2_DestroyActor`))

(fn `CheckHit`
  (params (Object :type "Actor Object Reference"))
  (if (`self.CanHit`)
    (bind _asmech (cast `Mech` Object)
      (:`then`
        (`Mech.Damage` _asmech (`self.Damage`) (`self.K2_GetActorLocation` _asmech)))
      (:`CastFailed`
        (bind _asthird_person_character (cast `/Game/Blueprints/Player/ThirdPersonCharacter` Object))
        (`/Game/Blueprints/Player/ThirdPersonCharacter.Kill` _asthird_person_character)))
    (set `self.CanHit` false)))

(fn `CheckHit_0`
  (bind _capsule (`self.Capsule`))
  (if (`self.CanHit`)
    (bind _asmech (cast `Mech` (`|GetArrayItem` (`PrimitiveComponent.GetOverlappingActors` _capsule "/Script/VerticalSlice.Mech")))
      (:`then`
        (`Mech.Damage` _asmech (`self.Damage`) (`self.K2_GetActorLocation` _asmech)))
      (:`CastFailed`
        (bind _asthird_person_character (cast `/Game/Blueprints/Player/ThirdPersonCharacter` (`|GetArrayItem` (`PrimitiveComponent.GetOverlappingActors` _capsule "/Game/Blueprints/Player/ThirdPersonCharacter.ThirdPersonCharacter_C"))))
        (`/Game/Blueprints/Player/ThirdPersonCharacter.Kill` _asthird_person_character)))
    (set `self.CanHit` false)))

(fn `UserConstructionScript`)