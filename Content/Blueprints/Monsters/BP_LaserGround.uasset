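; BP_LaserGround is a short-lived monster laser actor that exists in the world for a set Duration.
; On BeginPlay it starts a timer by function name that destroys the actor when it expires.
; An unconnected, never-run experiment line-traces forward up to MaxLength to stretch and offset the Cube hitbox to fit, with debug drawing and printing.
; No damage or overlap logic lives in this graph.
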(event `self.ReceiveBeginPlay`
  (`KismetSystemLibrary.K2_SetTimer` null "DestroyAfterXSeconds" (`self.Duration`)))

(event `DestroyAfterXSeconds`
  (`self.K2_DestroyActor`))

(fn `UserConstructionScript`)