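; BP_RockyJumpSmash is a short-lived area damage actor for Rocky's jump smash attack.
; On BeginPlay it spawns the slam particle effect, sizes a debug sphere mesh to the collision radius, and starts a self-destruct timer.
; Sphere overlap damages MechBoi2 or kills ThirdPersonCharacter, with a HasHit flag limiting it to one successful hit.
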(event `self.ReceiveBeginPlay`
  (bind _returnvalue (/ (`SphereComponent.SphereRadius` (`self.Sphere`)) 50.0))
  ;[1 1 1] Set Sphere Scale for Debugging
  (`SceneComponent.SetRelativeScale3D` (`self.SM_Sphere`) (`KismetMathLibrary.MakeVector` _returnvalue _returnvalue _returnvalue))
  (`KismetSystemLibrary.K2_SetTimer` null "DestroySelf" (`self.ActiveTime`))
  (`NiagaraFunctionLibrary.SpawnSystemAtLocation` "/Game/Effects/Niagra/P_RockyJumpSlam.P_RockyJumpSlam" (`self.K2_GetActorLocation`))
  (if (`self.Debug`)
    (`SceneComponent.SetVisibility` (`self.SM_Sphere`) true false)
    (else
      (`SceneComponent.SetVisibility` (`self.SM_Sphere`) false false))))

(event `DestroySelf`
  (`self.K2_DestroyActor`))

(event `CheckOverlap`)

(event `self.Sphere.OnComponentBeginOverlap`
  (params (OverlappedComponent :type "PrimitiveComponent Object Reference") (OtherActor :type "Actor Object Reference") (OtherComp :type "PrimitiveComponent Object Reference") (OtherBodyIndex :type Integer) (bFromSweep :type Boolean) (SweepResult :type "HitResult Structure (by ref)"))
  (`self.DamagePlayer` OtherActor))

(fn `DamagePlayer`
  (params (Object :type "Actor Object Reference"))
  ;[1 1 1] Make sure hasn't hit yet
  (if (not (`self.HasHit`))
    (bind _asmech_boi_2 (cast `/Game/Blueprints/Player/MechBoi2` (`local.Object`))
      (:`then`
        (`Mech.Damage` _asmech_boi_2 (`self.Damage`) (`self.K2_GetActorLocation` _asmech_boi_2)))
      (:`CastFailed`
        (bind _asthird_person_character (cast `/Game/Blueprints/Player/ThirdPersonCharacter` (`local.Object`)))
        (`/Game/Blueprints/Player/ThirdPersonCharacter.Kill` _asthird_person_character)))
    (set `self.HasHit` true)))

(fn `UserConstructionScript`)