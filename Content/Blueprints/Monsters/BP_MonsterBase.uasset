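; Base monster Blueprint that handles player sensing and weakspot-based damage with floating numbers.
; AI perception updates of a MechBoi2 actor write the sensed state to the CanSeePlayer blackboard key.
; DamageMonster calls DamageNumbers, which flags weakspot bone hits as crits and shows a damage widget at the monster's projected screen position.
; DamageNumbers then calls DamageMonster again with crit-scaled or base damage and no bone, forming a recursive loop.
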(event `self.ReceiveBeginPlay`)

(event `self.ReceiveActorBeginOverlap`
  (params (OtherActor :type "Actor Object Reference")))

(event `self.ReceiveTick`
  (params (DeltaSeconds :type "Float (single-precision)")))

(event `self.AIPerception.OnTargetPerceptionUpdated`
  (params (Actor :type "Actor Object Reference") (Stimulus :type "AIStimulus Structure"))
  (cast `/Game/Experimental/ThirdPersonCPP/Blueprints/MechBoi2` Actor)
  (`BlackboardComponent.SetValueAsBool` (`AIBlueprintHelperLibrary.GetBlackboard` null) "CanSeePlayer" (`.bSuccessfullySensed` (break `AIStimulus` Stimulus)))
  (`KismetSystemLibrary.PrintString` "Base"))

(event `self.DamageMonster`
  (params (_damage :type "Float (single-precision)") (_hitLoc :type "Vector Structure") (_boneHit :type Name))
  (`self.DamageNumbers` (`KismetStringLibrary.Conv_NameToString` _boneHit) _damage _hitLoc))

(fn `DamageNumbers`
  (params (BoneHit :type String) (BaseDamage :type "Float (double-precision)" :default 0.0) (HitLocation :type "Vector Structure"))
  (locals (IsCrit :type Boolean))
  (for _array_element (`self.WeakspotsScript`)
    ;[1 1 1] Check if weakspot is hit
    (if (`KismetStringLibrary.EqualEqual_StrStr` _array_element BoneHit)
      (set `local.IsCrit` true)
      (break)))
  (bind _returnvalue (`|CreateWidget` "/Game/UI/Widget_Damage1.Widget_Damage1_C" (`GameplayStatics.GetPlayerController` 0) (`local.IsCrit`) BaseDamage))
  (`UserWidget.AddToViewport` _returnvalue 0)
  (`UserWidget.SetPositionInViewport` _returnvalue (`GameplayStatics.ProjectWorldToScreen` (`GameplayStatics.GetPlayerController` 0) (`self.K2_GetActorLocation`)) true)
  (if (`local.IsCrit`)
    (`self.DamageMonster` (* (`self.CritMulti`) (`local.BaseDamage`)))
    (else
      (`self.DamageMonster` (`local.BaseDamage`))))
  (return))

(fn `UserConstructionScript`)