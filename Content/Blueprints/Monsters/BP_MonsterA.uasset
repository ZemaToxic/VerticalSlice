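; Leaping melee monster, built on a parent monster class, that swaps to horde AI controller and behavior tree in GM_HordeMode.
; A timer turns it toward the player, then flags the attack on the blackboard.
; StartCheckingHits launches it forward and loops head-socket sphere sweeps until one damages MechBoi2 or kills a ThirdPersonCharacter.
; Falling lateral friction drops to zero for the leap and is restored on landing or damage.
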(event `self.ReceiveBeginPlay`
  (`parent.ReceiveBeginPlay`)
  (cast `GM_HordeMode` (`GameplayStatics.GetGameMode`))
  (set `self.AIControllerClass` "/Game/AI/AIC_MonsterA_Horde.AIC_MonsterA_Horde_C")
  (set `self.BehaviorTreeComp` "/Game/AI/BT_MonsterA_Horde.BT_MonsterA_Horde"))

(event `SweepTest`
  (bind _returnvalue (`SceneComponent.GetSocketLocation` (`self.Mesh`) "SaberHead"))
  (bind _outhits (`KismetSystemLibrary.SphereTraceMulti` _returnvalue (+ _returnvalue (`self.GetActorForwardVector`)) 125.0 "TraceTypeQuery5"))
  (for _array_element _outhits
    (bind _asmech_boi_2 (cast `/Game/Blueprints/Player/MechBoi2` (`.HitActor` (`GameplayStatics.BreakHitResult` _array_element)))
      (:`then`
        (`Mech.Damage` _asmech_boi_2 (`self.damage`) (`.Location` (`GameplayStatics.BreakHitResult` _array_element))))
      (:`CastFailed`
        (bind _asthird_person_character (cast `/Game/Blueprints/Player/ThirdPersonCharacter` (`.HitActor` (`GameplayStatics.BreakHitResult` _array_element))))
        (`/Game/Blueprints/Player/ThirdPersonCharacter.Kill` _asthird_person_character)))
    (`self.StopCheckingHits`)
    (break)))

(event `StartCheckingHits`
  (`KismetSystemLibrary.K2_SetTimer` null "SweepTest" 0.02 true)
  (`self.Launch`))

(event `StopCheckingHits`
  (`KismetSystemLibrary.K2_PauseTimer` null "SweepTest"))

(event `self.DamageMonster`
  (params (_Damage :type "Float (single-precision)") (_HitLoc :type "Vector Structure") (_BoneHit :type Name) (_KnockbackForce :type "Float (single-precision)"))
  (set `CharacterMovementComponent.FallingLateralFriction` 4.0 (`self.CharacterMovement`))
  (`parent.DamageMonster` _Damage _HitLoc _BoneHit _KnockbackForce))

(event `RotateTowardsPlayer`
  (bind (_returnvalue_x _returnvalue_y) (`KismetMathLibrary.BreakVector` (`self.K2_GetActorLocation`)))
  (bind (_returnvalue_roll _returnvalue_pitch _returnvalue_yaw) (`KismetMathLibrary.BreakRotator` (`self.K2_GetActorRotation`)))
  (bind (_returnvalue_x_2 _returnvalue_y_2) (`KismetMathLibrary.BreakVector` (`self.K2_GetActorLocation` (`GameplayStatics.GetPlayerPawn` 0))))
  (bind (_returnvalue_roll_2 _returnvalue_pitch_2 _returnvalue_yaw_2) (`KismetMathLibrary.BreakRotator` (`KismetMathLibrary.FindLookAtRotation` (`KismetMathLibrary.MakeVector` _returnvalue_x _returnvalue_y) (`KismetMathLibrary.MakeVector` _returnvalue_x_2 _returnvalue_y_2))))
  (`MovementComponent.StopMovementImmediately` (`self.CharacterMovement`))
  (`self.K2_SetActorRotation` (`KismetMathLibrary.RInterpTo_Constant` (`self.K2_GetActorRotation`) (`KismetMathLibrary.MakeRotator` 0.0 0.0 _returnvalue_yaw_2) 0.01 750.0))
  (if (<= (`KismetMathLibrary.Abs` (- _returnvalue_yaw_2 _returnvalue_yaw)) 10.0)
    (`KismetSystemLibrary.K2_PauseTimer` null "RotateTowardsPlayer")
    (`self.LeapAttack`)))

(event `StartRotatingTowardsPlayer`
  (`KismetSystemLibrary.K2_SetTimer` null "RotateTowardsPlayer" 0.01 true))

(event `self.OnLanded`
  (params (Hit :type "HitResult Structure (by ref)"))
  (set `CharacterMovementComponent.FallingLateralFriction` 4.0 (`self.CharacterMovement`)))

(fn `Launch`
  (bind (_returnvalue_x _returnvalue_y) (`KismetMathLibrary.BreakVector` (* (`self.GetActorForwardVector`) (`self.LeapForce`))))
  (set `CharacterMovementComponent.FallingLateralFriction` 0.0 (`self.CharacterMovement`))
  (`self.LaunchCharacter` (`KismetMathLibrary.MakeVector` _returnvalue_x _returnvalue_y (`self.LeapZForce`)) true true))

(fn `LeapAttack`
  (`BlackboardComponent.SetValueAsBool` (`AIBlueprintHelperLibrary.GetBlackboard` null) "Attacking" true)
  (`BlackboardComponent.SetValueAsBool` (`AIBlueprintHelperLibrary.GetBlackboard` null) "IsInAttackRange" false))

(fn `LeapCheck`)

(fn `UserConstructionScript`
  (`parent.UserConstructionScript`))