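; Monster C: a charging melee enemy with two arm hitboxes and an armor plate.
; While an arm's hit flag is set, its overlaps damage MechBoi2 and clear both flags, or kill ThirdPersonCharacter outright.
; Other overlaps and all arm collisions run CheckCrash, which sets blackboard StopCharge if charging into anything but monsters, players or drops.
; A looping BeginPlay timer retries until BPArmorBase is valid, then hands it the plate mesh.
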(event `self.ReceiveBeginPlay`
  (bind _returnvalue (`KismetSystemLibrary.K2_SetTimerDelegate` (delegate `Set SMRef`) 0.01 true)))

(event `Set SMRef`
  (if (`KismetSystemLibrary.IsValid` (`self.BP_ArmorBase`))
    (set `ArmorBase.SMRef` (`self.SM_ArmorPlate`) (`self.BP_ArmorBase`))
    (`KismetSystemLibrary.K2_ClearAndInvalidateTimerHandle` (stale `self.ReceiveBeginPlay` _returnvalue))))

(event `self.LeftArm.OnComponentBeginOverlap`
  (params (OverlappedComponent :type "PrimitiveComponent Object Reference") (OtherActor :type "Actor Object Reference") (OtherComp :type "PrimitiveComponent Object Reference") (OtherBodyIndex :type Integer) (bFromSweep :type Boolean) (SweepResult :type "HitResult Structure (by ref)"))
  (if (`self.LeftArmHit`)
    (bind _asmech_boi_2 (cast `/Game/Blueprints/Player/MechBoi2` OtherActor)
      (:`then`
        (`Mech.Damage` _asmech_boi_2 (`self.damage`) (0.0 0.0 0.0))
        (`self.StopHits` :!label _label))
      (:`CastFailed`
        (bind _asthird_person_character (cast `/Game/Blueprints/Player/ThirdPersonCharacter` OtherActor)
          (:`then`
            (`/Game/Blueprints/Player/ThirdPersonCharacter.Kill` _asthird_person_character))
          (:`CastFailed`
            (`self.CheckCrash` OtherActor)))))))

(event `self.RightArm.OnComponentBeginOverlap`
  (params (OverlappedComponent :type "PrimitiveComponent Object Reference") (OtherActor :type "Actor Object Reference") (OtherComp :type "PrimitiveComponent Object Reference") (OtherBodyIndex :type Integer) (bFromSweep :type Boolean) (SweepResult :type "HitResult Structure (by ref)"))
  (if (`self.RightArmHit`)
    (bind _asmech_boi_2 (cast `/Game/Blueprints/Player/MechBoi2` OtherActor)
      (:`then`
        (`Mech.Damage` _asmech_boi_2 (`self.damage`) (0.0 0.0 0.0))
        (goto _label))
      (:`CastFailed`
        (bind _asthird_person_character (cast `/Game/Blueprints/Player/ThirdPersonCharacter` OtherActor)
          (:`then`
            (`/Game/Blueprints/Player/ThirdPersonCharacter.Kill` _asthird_person_character))
          (:`CastFailed`
            (`self.CheckCrash` OtherActor)))))))

(event `self.RightArm.OnComponentHit`
  (params (HitComponent :type "PrimitiveComponent Object Reference") (OtherActor :type "Actor Object Reference") (OtherComp :type "PrimitiveComponent Object Reference") (NormalImpulse :type "Vector Structure") (Hit :type "HitResult Structure (by ref)"))
  (`self.CheckCrash` OtherActor))

(event `self.LeftArm.OnComponentHit`
  (params (HitComponent :type "PrimitiveComponent Object Reference") (OtherActor :type "Actor Object Reference") (OtherComp :type "PrimitiveComponent Object Reference") (NormalImpulse :type "Vector Structure") (Hit :type "HitResult Structure (by ref)"))
  (`self.CheckCrash` OtherActor))

(fn `CheckCrash`
  (params (Object :type "Object Object Reference"))
  (if (`BlackboardComponent.GetValueAsBool` (`AIBlueprintHelperLibrary.GetBlackboard` null) "IsCharging")
    (cast `/Game/Blueprints/Monsters/BP_MonsterBase` Object
      (:`CastFailed`
        (cast `/Game/Blueprints/Player/MechBoi2` Object
          (:`CastFailed`
            (cast `/Game/Blueprints/Player/ThirdPersonCharacter` Object
              (:`CastFailed`
                (cast `/Game/Blueprints/Drops/BP_DropsBase` Object
                  (:`CastFailed`
                    (`BlackboardComponent.SetValueAsBool` (`AIBlueprintHelperLibrary.GetBlackboard` null) "StopCharge" true)))))))))))

(fn `SpawnDrops`
  (`parent.SpawnDrops`))

(fn `StopHits`
  (set `self.RightArmHit` false)
  (set `self.LeftArmHit` false))

(fn `UserConstructionScript`
  (`parent.UserConstructionScript`))