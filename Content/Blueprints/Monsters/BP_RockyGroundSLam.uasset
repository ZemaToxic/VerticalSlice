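; BP_RockyGroundSlam is a monster ground-slam hazard that advances as a chain of explosions, damaging Mechs and killing ThirdPersonCharacters.
; Each instance sizes its overlap box from a per-iteration width, then on a timer spawns the next instance ahead until MaxIterations.
; HasHit limits each segment to one victim and disarms it shortly before self-destruction.
; SpawnFX scales effect count with width but is not called in this graph.
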(event `self.ReceiveBeginPlay`
  (bind _box (`self.Box`))
  (bind (_returnvalue_x _returnvalue_y _returnvalue_z) (`KismetMathLibrary.BreakVector` (`SceneComponent.K2_GetComponentScale` _box)))
  (`SceneComponent.SetWorldScale3D` _box (`KismetMathLibrary.MakeVector` _returnvalue_x (`|GetArrayItem` (`self.Widths`) (`self.CurrentIteration`)) _returnvalue_z))
  (`KismetSystemLibrary.K2_SetTimer` null "DestroySelf" (`self.ActiveTime`))
  (`self.CheckSpawnRequired`))

(event `DestroySelf`
  (set `self.HasHit` true)
  (`KismetSystemLibrary.Delay` 0.5)
  (`self.K2_DestroyActor`))

(event `CheckSpawnRequired`
  (if (< (`self.CurrentIteration`) (- (`self.MaxIterations`) 1))
    (`KismetSystemLibrary.K2_SetTimer` null "SpawnNext" (`self.DelayBetweenExplosions`))))

(event `SpawnNext`
  (`|SpawnActorFromClass` "BP_RockyGroundSlam_C" (`KismetMathLibrary.MakeTransform` (+ (* (`self.GetActorForwardVector`) (`self.DistanceBetweenExplosions`)) (`self.K2_GetActorLocation`)) (`self.K2_GetActorRotation`)) "Undefined" "OverrideRootScale" null (+ (`self.CurrentIteration`) 1) null))

(event `self.Box.OnComponentBeginOverlap`
  (params (OverlappedComponent :type "PrimitiveComponent Object Reference") (OtherActor :type "Actor Object Reference") (OtherComp :type "PrimitiveComponent Object Reference") (OtherBodyIndex :type Integer) (bFromSweep :type Boolean) (SweepResult :type "HitResult Structure (by ref)"))
  (`self.CheckDamage` OtherActor))

(fn `CheckDamage`
  (params (Object :type "Actor Object Reference"))
  (if (not (`self.HasHit`))
    (bind _asmech (cast `Mech` Object)
      (:`then`
        (`Mech.Damage` _asmech (`self.Damage`) (`self.K2_GetActorLocation` _asmech)))
      (:`CastFailed`
        (bind _asthird_person_character (cast `/Game/Blueprints/Player/ThirdPersonCharacter` Object))
        (`/Game/Blueprints/Player/ThirdPersonCharacter.Kill` _asthird_person_character)))
    (set `self.HasHit` true)))

(fn `SpawnFX`
  (for _ (range (+ (`KismetMathLibrary.FCeil` (/ (`|GetArrayItem` (`self.Widths`) (`self.CurrentIteration`)) 10.0)) 1))
    (`NiagaraFunctionLibrary.SpawnSystemAtLocation` null (0.0 0.0 0.0) (`self.K2_GetActorRotation`))))

(fn `UserConstructionScript`)