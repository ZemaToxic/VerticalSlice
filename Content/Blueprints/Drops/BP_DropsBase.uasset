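; BP_DropsBase is a base drop actor that flies toward the player and awards parts on pickup.
; A magnet sphere overlap or a looping range-check timer, which covers drops spawned within range, restarts a timeline.
; Each timeline update interpolates the location toward the player, plus a track offset.
; Overlapping the pickup sphere adds one part of its DropType through BP_GM_Base, then destroys the drop.
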(event `self.ReceiveBeginPlay`
  (`KismetSystemLibrary.K2_SetTimerDelegate` (delegate `ShouldPickup`) 0.5 true))

(event `ShouldPickup`
  ;[1 1 1] For when the object is already within range of player when it is spawned
  (bind _returnvalue (`self.CheckInRange`))
  (if _returnvalue
    (bind (_direction _newtrack_0) (`Timeline|Timeline_0` :!via `PlayFromStart` :!label _label)
      (:`Update`
        (`self.K2_SetActorLocation` (+ _newtrack_0 (`KismetMathLibrary.VInterpTo` (.location (`self.GetTransform`)) (`self.K2_GetActorLocation` (`GameplayStatics.GetPlayerCharacter` 0)) (`GameplayStatics.GetWorldDeltaSeconds`) 5.0)))))))

(event `self.MagnetSphereComp.OnComponentBeginOverlap`
  (params (OverlappedComponent :type "PrimitiveComponent Object Reference") (OtherActor :type "Actor Object Reference") (OtherComp :type "PrimitiveComponent Object Reference") (OtherBodyIndex :type Integer) (bFromSweep :type Boolean) (SweepResult :type "HitResult Structure (by ref)"))
  (if (== OtherActor (`GameplayStatics.GetPlayerCharacter` 0))
    (goto _label :!via `PlayFromStart`)))

(event `self.PickupSphereComp.OnComponentBeginOverlap`
  (params (OverlappedComponent :type "PrimitiveComponent Object Reference") (OtherActor :type "Actor Object Reference") (OtherComp :type "PrimitiveComponent Object Reference") (OtherBodyIndex :type Integer) (bFromSweep :type Boolean) (SweepResult :type "HitResult Structure (by ref)"))
  (if (== OtherActor (`GameplayStatics.GetPlayerCharacter` 0))
    (bind _asbp_gm_base (cast `/Game/Blueprints/BP_GM_Base` (`GameplayStatics.GetGameMode`)))
    (`GM_Base.AddParts` _asbp_gm_base (`self.DropType`) 1)
    (`self.K2_DestroyActor`)))

(fn `UserConstructionScript`)