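; BP_Trail is a short-lived effect actor moved by a projectile movement component, presumably to draw a trail.
; On BeginPlay it rescales its current velocity direction to StartSpeed and travels for AliveDuration.
; It then stops movement and waits one second before destroying itself.
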(event `self.ReceiveBeginPlay`
  (bind _projectilemovement (`self.ProjectileMovement`))
  (set `MovementComponent.Velocity` (* (`KismetMathLibrary.Normal` (`self.GetVelocity`)) (`self.startSpeed`)) (`self.ProjectileMovement`))
  (`KismetSystemLibrary.Delay` (`self.aliveDuration`))
  (set `MovementComponent.Velocity` (0.0 0.0 0.0) _projectilemovement)
  (`MovementComponent.StopMovementImmediately` _projectilemovement)
  (`KismetSystemLibrary.Delay` 1.0)
  (`self.K2_DestroyActor`))

(fn `UserConstructionScript`)